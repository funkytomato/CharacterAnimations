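; Civilian character Blueprint that plays punch and kick attacks from input, plus knockdown and crowd-style emotes such as cheer, wave and yell from custom events.
; Each action, blocked while falling or by its own busy flag, disables movement, plays a random montage, waits its length, then restores walking.
; The overlap handler only casts to MasterCharacter, and a hit reaction with groan and health loss is left unconnected.
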(event `self.ReceiveBeginPlay`
  (`parent.ReceiveBeginPlay`))

(event `self.ReceiveActorBeginOverlap`
  (params (OtherActor :type "Actor Object Reference"))
  ;[1 1 1] Interact with overlapped actor
  (`parent.ReceiveActorBeginOverlap` OtherActor)
  (cast `/Game/MyContent/Blueprints/Characters/MasterCharacter` OtherActor))

(event `InputAction|Punch`
  (params (Key :type "Key Structure"))
  (bind _charactermovement (`self.CharacterMovement`))
  ;[1 1 1] Punch Kick or something
  (:`Pressed`
    (if (`NavMovementComponent.IsFalling` (`self.CharacterMovement`))
      _
      (elif (not (`self.isPunching?`))
        (set `self.isPunching?` true)
        (`CharacterMovementComponent.DisableMovement` _charactermovement)
        (bind _returnvalue (`self.PlayAnimMontage` (`|GetArrayItem` (`self.PunchAnimMontages`) (`KismetMathLibrary.RandomIntegerInRange` 0 5))))
        (`KismetSystemLibrary.Delay` _returnvalue)
        (`CharacterMovementComponent.SetMovementMode` _charactermovement "MOVE_Walking" 0)
        (set `self.isPunching?` false)))))

(event `InputAction|Kick`
  (params (Key :type "Key Structure"))
  (bind _charactermovement (`self.CharacterMovement`))
  ;[1 1 1] Kick
  (:`Pressed`
    (if (`NavMovementComponent.IsFalling` (`self.CharacterMovement`))
      _
      (elif (not (`self.IsKicking?`))
        (set `self.IsKicking?` true)
        (`CharacterMovementComponent.DisableMovement` _charactermovement)
        (bind _returnvalue (`self.PlayAnimMontage` (`|GetArrayItem` (`self.KickingAnimMontages`) (`KismetMathLibrary.RandomIntegerInRange` 0 2))))
        (`KismetSystemLibrary.Delay` _returnvalue)
        (`CharacterMovementComponent.SetMovementMode` _charactermovement "MOVE_Walking" 0)
        (set `self.IsKicking?` false)))))

(event `Knockdown`
  (bind _charactermovement (`self.CharacterMovement`))
  ;[1 1 1] Knockdown
  (if (`NavMovementComponent.IsFalling` (`self.CharacterMovement`))
    _
    (elif (not (`self.IsKnockedDown?`))
      (set `self.IsKnockedDown?` true)
      (`CharacterMovementComponent.DisableMovement` _charactermovement)
      (bind _returnvalue (`self.PlayAnimMontage` (`|GetArrayItem` (`self.KnockdownAnimMontages`) (`KismetMathLibrary.RandomIntegerInRange` 0 2))))
      (`KismetSystemLibrary.Delay` _returnvalue)
      (`CharacterMovementComponent.SetMovementMode` _charactermovement "MOVE_Walking" 0)
      (set `self.IsKnockedDown?` false))))

(event `Cheer`
  (bind _charactermovement (`self.CharacterMovement`))
  ;[1 1 1] Cheer
  (if (`NavMovementComponent.IsFalling` (`self.CharacterMovement`))
    _
    (elif (not (`self.IsCheering?`))
      (set `self.IsCheering?` true)
      (`CharacterMovementComponent.DisableMovement` _charactermovement)
      (bind _returnvalue (`self.PlayAnimMontage` (`|GetArrayItem` (`self.CheeringMontages`) (`KismetMathLibrary.RandomIntegerInRange` 0 2))))
      (`KismetSystemLibrary.Delay` _returnvalue)
      (`CharacterMovementComponent.SetMovementMode` _charactermovement "MOVE_Walking" 0)
      (set `self.IsCheering?` false))))

(event `Fistpump`
  (bind _charactermovement (`self.CharacterMovement`))
  ;[1 1 1] Fistpumping
  (if (`NavMovementComponent.IsFalling` (`self.CharacterMovement`))
    _
    (elif (not (`self.IsFistpumping?`))
      (set `self.IsFistpumping?` true)
      (`CharacterMovementComponent.DisableMovement` _charactermovement)
      (bind _returnvalue (`self.PlayAnimMontage` (`|GetArrayItem` (`self.FistpumpMontages`) (`KismetMathLibrary.RandomIntegerInRange` 0 2))))
      (`KismetSystemLibrary.Delay` _returnvalue)
      (`CharacterMovementComponent.SetMovementMode` _charactermovement "MOVE_Walking" 0)
      (set `self.IsFistpumping?` false))))

(event `LeanForwardYell`
  (bind _charactermovement (`self.CharacterMovement`))
  ;[1 1 1] Lean Forward Yell
  (if (`NavMovementComponent.IsFalling` (`self.CharacterMovement`))
    _
    (elif (not (`self.isLeaningForward?`))
      (set `self.isLeaningForward?` true)
      (`CharacterMovementComponent.DisableMovement` _charactermovement)
      (bind _returnvalue (`self.PlayAnimMontage` (`|GetArrayItem` (`self.LeaningForwardMontages`) (`KismetMathLibrary.RandomIntegerInRange` 0 2))))
      (`KismetSystemLibrary.Delay` _returnvalue)
      (`CharacterMovementComponent.SetMovementMode` _charactermovement "MOVE_Walking" 0)
      (set `self.isLeaningForward?` false))))

(event `RadCheer`
  (bind _charactermovement (`self.CharacterMovement`))
  ;[1 1 1] Metal/Radical Cheer
  (if (`NavMovementComponent.IsFalling` (`self.CharacterMovement`))
    _
    (elif (not (`self.IsMetalCheer?`))
      (set `self.IsMetalCheer?` true)
      (`CharacterMovementComponent.DisableMovement` _charactermovement)
      (bind _returnvalue (`self.PlayAnimMontage` (`|GetArrayItem` (`self.MetalMontages`) (`KismetMathLibrary.RandomIntegerInRange` 0 2))))
      (`KismetSystemLibrary.Delay` _returnvalue)
      (`CharacterMovementComponent.SetMovementMode` _charactermovement "MOVE_Walking" 0)
      (set `self.IsMetalCheer?` false))))

(event `Pointing`
  (bind _charactermovement (`self.CharacterMovement`))
  (if (`NavMovementComponent.IsFalling` (`self.CharacterMovement`))
    _
    (elif (not (`self.IsPointing?`))
      (set `self.IsPointing?` true)
      (`CharacterMovementComponent.DisableMovement` _charactermovement)
      (bind _returnvalue (`self.PlayAnimMontage` (`|GetArrayItem` (`self.PointingMontages`) (`KismetMathLibrary.RandomIntegerInRange` 0 2))))
      (`KismetSystemLibrary.Delay` _returnvalue)
      (`CharacterMovementComponent.SetMovementMode` _charactermovement "MOVE_Walking" 0)
      (set `self.IsPointing?` false))))

(event `Slouch`
  (bind _charactermovement (`self.CharacterMovement`))
  (if (`NavMovementComponent.IsFalling` (`self.CharacterMovement`))
    _
    (elif (not (`self.IsSlouching?`))
      (set `self.IsSlouching?` true)
      (`CharacterMovementComponent.DisableMovement` _charactermovement)
      (bind _returnvalue (`self.PlayAnimMontage` (`|GetArrayItem` (`self.SlouchingMontages`) (`KismetMathLibrary.RandomIntegerInRange` 0 2))))
      (`KismetSystemLibrary.Delay` _returnvalue)
      (`CharacterMovementComponent.SetMovementMode` _charactermovement "MOVE_Walking" 0)
      (set `self.IsSlouching?` false))))

(event `ThumbsDown`
  (bind _charactermovement (`self.CharacterMovement`))
  (if (`NavMovementComponent.IsFalling` (`self.CharacterMovement`))
    _
    (elif (not (`self.IsThumbsDown?`))
      (set `self.IsThumbsDown?` true)
      (`CharacterMovementComponent.DisableMovement` _charactermovement)
      (bind _returnvalue (`self.PlayAnimMontage` (`|GetArrayItem` (`self.ThumbsDownMontages`) (`KismetMathLibrary.RandomIntegerInRange` 0 2))))
      (`KismetSystemLibrary.Delay` _returnvalue)
      (`CharacterMovementComponent.SetMovementMode` _charactermovement "MOVE_Walking" 0)
      (set `self.IsThumbsDown?` false))))

(event `ThumbsUp`
  (bind _charactermovement (`self.CharacterMovement`))
  (if (`NavMovementComponent.IsFalling` (`self.CharacterMovement`))
    _
    (elif (not (`self.isThumbsUp?`))
      (set `self.isThumbsUp?` true)
      (`CharacterMovementComponent.DisableMovement` _charactermovement)
      (bind _returnvalue (`self.PlayAnimMontage` (`|GetArrayItem` (`self.ThumbsUpMontages`) (`KismetMathLibrary.RandomIntegerInRange` 0 2))))
      (`KismetSystemLibrary.Delay` _returnvalue)
      (`CharacterMovementComponent.SetMovementMode` _charactermovement "MOVE_Walking" 0)
      (set `self.isThumbsUp?` false))))

(event `Wave`
  (bind _charactermovement (`self.CharacterMovement`))
  (if (`NavMovementComponent.IsFalling` (`self.CharacterMovement`))
    _
    (elif (not (`self.IsWaving?`))
      (set `self.IsWaving?` true)
      (`CharacterMovementComponent.DisableMovement` _charactermovement)
      (bind _returnvalue (`self.PlayAnimMontage` (`|GetArrayItem` (`self.WavingMontages`) (`KismetMathLibrary.RandomIntegerInRange` 0 2))))
      (`KismetSystemLibrary.Delay` _returnvalue)
      (`CharacterMovementComponent.SetMovementMode` _charactermovement "MOVE_Walking" 0)
      (set `self.IsWaving?` false))))

(event `Yell`
  (bind _charactermovement (`self.CharacterMovement`))
  (if (`NavMovementComponent.IsFalling` (`self.CharacterMovement`))
    _
    (elif (not (`self.IsYelling?`))
      (set `self.IsYelling?` true)
      (`CharacterMovementComponent.DisableMovement` _charactermovement)
      (bind _returnvalue (`self.PlayAnimMontage` (`|GetArrayItem` (`self.YellingMontages`) (`KismetMathLibrary.RandomIntegerInRange` 0 2))))
      (`KismetSystemLibrary.Delay` _returnvalue)
      (`CharacterMovementComponent.SetMovementMode` _charactermovement "MOVE_Walking" 0)
      (set `self.IsYelling?` false))))

(fn `UserConstructionScript`
  (`parent.UserConstructionScript`))