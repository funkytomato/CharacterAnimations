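; Swordsman character Blueprint that performs melee actions: attack, block, dodge, victory pose and taunt.
; Each input action plays a random montage from its own array, guarded by an airborne check and its own busy flag.
; Movement is disabled for the montage's returned duration via Delay, then walking is restored; blocking also sets IsDefending.
; All actions except attack are also exposed as events for triggering without input.
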(event `self.ReceiveBeginPlay`
  (`parent.ReceiveBeginPlay`)
  (bind _asswordsman_anim_bp (cast `/Game/MyContent/Blueprints/Characters/Swordsman_AnimBP` (`SkeletalMeshComponent.GetAnimInstance` (`self.Mesh`))))
  (set `self.AnimInstance` _asswordsman_anim_bp))

(event `self.ReceiveActorBeginOverlap`
  (params (OtherActor :type "Actor Object Reference"))
  (`parent.ReceiveActorBeginOverlap` OtherActor))

(event `InputAction|Attack`
  (params (Key :type "Key Structure"))
  (bind _charactermovement (`self.CharacterMovement`))
  ;[1 1 1] Attack Opponent
  (:`Pressed`
    (if (`NavMovementComponent.IsFalling` (`self.CharacterMovement`))
      _
      (elif (not (`self.IsAttacking?`))
        (set `self.IsAttacking?` true)
        (`CharacterMovementComponent.DisableMovement` _charactermovement)
        (bind _returnvalue (`self.PlayAnimMontage` (`|GetArrayItem` (`self.SwordAttackMontages`) (`KismetMathLibrary.RandomIntegerInRange` 0 49))))
        (`KismetSystemLibrary.Delay` _returnvalue)
        (`CharacterMovementComponent.SetMovementMode` _charactermovement "MOVE_Walking" 0)
        (set `self.IsAttacking?` false)))))

(event `InputAction|Block`
  (params (Key :type "Key Structure"))
  (bind _charactermovement (`self.CharacterMovement`))
  ;[1 1 1] Parry Opponents Attack
  (:`Pressed`
    (if (`NavMovementComponent.IsFalling` (`self.CharacterMovement`)) :!label _label
      _
      (elif (not (`self.IsBlocking?`))
        (set `self.IsDefending?` true)
        (set `self.IsBlocking?` true)
        (`CharacterMovementComponent.DisableMovement` _charactermovement)
        (bind _returnvalue (`self.PlayAnimMontage` (`|GetArrayItem` (`self.BlockingMontages`) (`KismetMathLibrary.RandomIntegerInRange` 0 6))))
        (`KismetSystemLibrary.Delay` _returnvalue)
        (`CharacterMovementComponent.SetMovementMode` _charactermovement "MOVE_Walking" 0)
        (set `self.IsBlocking?` false)
        (set `self.IsDefending?` false)))))

(event `Block`
  ;[1 1 1] Parry Opponents Attack
  (goto _label))

(event `Dodge`
  (bind _charactermovement (`self.CharacterMovement`))
  ;[1 1 1] Evade/Dodge Opponents Attack
  (if (`NavMovementComponent.IsFalling` (`self.CharacterMovement`)) :!label _label_2
    _
    (elif (not (`self.IsEvading?`))
      (set `self.IsEvading?` true)
      (`CharacterMovementComponent.DisableMovement` _charactermovement)
      (bind _returnvalue (`self.PlayAnimMontage` (`|GetArrayItem` (`self.EvadeMontages`) (`KismetMathLibrary.RandomIntegerInRange` 0 10))))
      (`KismetSystemLibrary.Delay` _returnvalue)
      (`CharacterMovementComponent.SetMovementMode` _charactermovement "MOVE_Walking" 0)
      (set `self.IsEvading?` false))))

(event `InputAction|Dodge`
  (params (Key :type "Key Structure"))
  ;[1 1 1] Evade/Dodge Opponents Attack
  (:`Pressed`
    (goto _label_2)))

(event `InputAction|Victory`
  (params (Key :type "Key Structure"))
  (bind _charactermovement (`self.CharacterMovement`))
  ;[1 1 1] Victory Pose
  (:`Pressed`
    (if (`NavMovementComponent.IsFalling` (`self.CharacterMovement`)) :!label _label_3
      _
      (elif (not (`self.IsVictory?`))
        (set `self.IsVictory?` true)
        (`CharacterMovementComponent.DisableMovement` _charactermovement)
        (bind _returnvalue (`self.PlayAnimMontage` (`|GetArrayItem` (`self.VictoryMontages`) (`KismetMathLibrary.RandomIntegerInRange` 0 2))))
        (`KismetSystemLibrary.Delay` _returnvalue)
        (`CharacterMovementComponent.SetMovementMode` _charactermovement "MOVE_Walking" 0)
        (set `self.IsVictory?` false)))))

(event `Victory`
  ;[1 1 1] Victory Pose
  (goto _label_3))

(event `InputAction|Taunt`
  (params (Key :type "Key Structure"))
  (bind _charactermovement (`self.CharacterMovement`))
  ;[1 1 1] Taunt Opponent
  (:`Pressed`
    (if (`NavMovementComponent.IsFalling` (`self.CharacterMovement`)) :!label _label_4
      _
      (elif (not (`self.IsTaunting?`))
        (set `self.IsTaunting?` true)
        (`CharacterMovementComponent.DisableMovement` _charactermovement)
        (bind _returnvalue (`self.PlayAnimMontage` (`|GetArrayItem` (`self.TauntMontages`) (`KismetMathLibrary.RandomIntegerInRange` 0 10))))
        (`KismetSystemLibrary.Delay` _returnvalue)
        (`CharacterMovementComponent.SetMovementMode` _charactermovement "MOVE_Walking" 0)
        (set `self.IsTaunting?` false)))))

(event `Taunt`
  ;[1 1 1] Taunt Opponent
  (goto _label_4))

(fn `UserConstructionScript`
  (`parent.UserConstructionScript`))