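; DrunkCivilian is a drunk civilian character that toggles between fallen and standing states via the FallOverGetUp input.
; BeginPlay caches its DrunkCivilian_AnimBP instance.
; A FlipFlop plays the same get-up montage on both presses, waits for its length, then sets IsCrouching true or false.
; The get-up branch adds a short delay before the montage and prints a debug message afterward.
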(event `self.ReceiveBeginPlay`
  ;[1 1 1] BefginPlay - Set Anim Instance
  (`parent.ReceiveBeginPlay`)
  (bind _asdrunk_civilian_anim_bp (cast `/Game/MyContent/Blueprints/Characters/DrunkCivilian_AnimBP` (`SkeletalMeshComponent.GetAnimInstance` (`self.Mesh`))))
  (set `self.AnimInstanceRef` _asdrunk_civilian_anim_bp))

(event `self.ReceiveActorBeginOverlap`
  (params (OtherActor :type "Actor Object Reference"))
  (`parent.ReceiveActorBeginOverlap` OtherActor))

(event `InputAction|FallOverGetUp`
  (params (Key :type "Key Structure"))
  (:`Pressed`
    (`/Engine/EditorBlueprintResources/StandardMacros.FlipFlop`
      (:`A`
        (bind _returnvalue (`self.PlayAnimMontage` "/Game/MyContent/Animations/DrunkMan/Anim_Drunk_Man_Up_Montage.Anim_Drunk_Man_Up_Montage"))
        (`KismetSystemLibrary.Delay` _returnvalue)
        (set `self.IsCrouching` true))
      (:`B`
        (`KismetSystemLibrary.Delay` 1.0)
        (bind _returnvalue_2 (`self.PlayAnimMontage` "/Game/MyContent/Animations/DrunkMan/Anim_Drunk_Man_Up_Montage.Anim_Drunk_Man_Up_Montage"))
        (`KismetSystemLibrary.Delay` _returnvalue_2)
        (set `self.IsCrouching` false)
        (`KismetSystemLibrary.PrintString` "Getting up")))))

(fn `UserConstructionScript`
  (`parent.UserConstructionScript`))