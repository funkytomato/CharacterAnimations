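; PhysicalAnim_CBP is a component that gives a MasterCharacter partial physical animation using a hit reaction profile.
; On BeginPlay it adds a PhysicalAnimationComponent to its owner and binds it to the character mesh.
; TogglePhysicalAnimation simulates bodies below the pelvis bone, excluding it, applies HitReactionProfile and blends physics halfway with animation.
; Despite its name, the toggle event only switches the effect on.
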(event `self.ReceiveBeginPlay`
  (bind _returnvalue (`|AddComponentByClass` (`self.GetOwner`) "/Script/Engine.PhysicalAnimationComponent"))
  (bind _output_get (set `self.PhysicalAnimComp` _returnvalue))
  (bind _asmaster_character (cast `/Game/MyContent/Blueprints/Characters/MasterCharacter` (`self.GetOwner`)))
  (bind _mesh (`Character.Mesh` _asmaster_character))
  (`PhysicalAnimationComponent.SetSkeletalMeshComponent` _output_get _mesh)
  (set `self. MyMesh` _mesh))

(event `TogglePhysicalAnimation`
  (bind _physicalanimcomp (`self.PhysicalAnimComp`))
  (`SkeletalMeshComponent.SetAllBodiesBelowSimulatePhysics` (`self. MyMesh`) "Pelvis" true false)
  (`PhysicalAnimationComponent.ApplyPhysicalAnimationProfileBelow` _physicalanimcomp "Pelvis" "HitReactionProfile" false false)
  (`PhysicalAnimationComponent.SetStrengthMultiplyer` _physicalanimcomp 1.0)
  (`SkeletalMeshComponent.SetAllBodiesBelowPhysicsBlendWeight` (`self. MyMesh`) "Pelvis" 0.5 false true))