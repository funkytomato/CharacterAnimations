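; CloseCombatCharacter is a melee character Blueprint that reacts to being punched by another character of the same class.
; When a punching CloseCombatCharacter begins overlapping it, it plays an impact groan and a random hit montage, then applies damage to itself once the montage length elapses.
; Punch logic that locks movement during a random punch montage is present but disconnected, so it never runs.
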(event `self.ReceiveActorBeginOverlap`
  (params (OtherActor :type "Actor Object Reference"))
  ;[1 1 1] Hit
  (bind _asclose_combat_character (cast `/Game/MyContent/Blueprints/Characters/CloseCombatCharacter` OtherActor))
  (if (`/Game/MyContent/Blueprints/Characters/UnarmedCombatCharacter.isPunching?` _asclose_combat_character)
    (`GameplayStatics.PlaySoundAtLocation` "/Game/MyContent/Audio/GroanImpact_Cue.GroanImpact_Cue" (`self.K2_GetActorLocation`) (struct) 1.0 1.0 0.0 null null null)
    (bind _returnvalue (`self.PlayAnimMontage` (`|GetArrayItem` (`self.HitAnimMontage`) (`KismetMathLibrary.RandomIntegerInRange` 0 8))))
    (`KismetSystemLibrary.Delay` _returnvalue)
    (`GameplayStatics.ApplyDamage` self 5.0 null _asclose_combat_character "/Script/Engine.DamageType")))

(event `self.ReceiveBeginPlay`
  ;[1 1 1] BeginPlay
  (`parent.ReceiveBeginPlay`))

(event `InputAction|Punch`
  (params (Key :type "Key Structure"))
  ;[1 1 1] Punch
)

(fn `UserConstructionScript`
  (`parent.UserConstructionScript`))