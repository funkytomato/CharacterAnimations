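; Gladiator character Blueprint that carries a shield and builds on a parent class.
; The construction script snaps the shield child actor component to the mesh's ShieldSocket.
; BeginPlay runs the parent logic, then caches the Gladiator animation instance and the spawned ShieldMaster_BP shield, stopping if either cast fails.
; Overlap events pass straight through to the parent.
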(event `self.ReceiveBeginPlay`
  (`parent.ReceiveBeginPlay`)
  (bind _asgladiator_anim_bp (cast `/Game/MyContent/Blueprints/Characters/Gladiator_AnimBP` (`SkeletalMeshComponent.GetAnimInstance` (`self.Mesh`))))
  (set `self.AnimInstance` _asgladiator_anim_bp)
  (bind _asshield_master_bp (cast `/Game/MyContent/Melee/ShieldMaster_BP` (`ChildActorComponent.ChildActor` (`self.ShieldComponent`))))
  (set `self.CurrentShield` _asshield_master_bp))

(event `self.ReceiveActorBeginOverlap`
  (params (OtherActor :type "Actor Object Reference"))
  (`parent.ReceiveActorBeginOverlap` OtherActor))

(fn `UserConstructionScript`
  (`parent.UserConstructionScript`)
  (`SceneComponent.K2_AttachToComponent` (`self.ShieldComponent`) (`self.Mesh`) "ShieldSocket" "SnapToTarget" "SnapToTarget" "SnapToTarget" true))