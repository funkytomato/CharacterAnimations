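; Unarmed combat character Blueprint providing punches, kicks, dodges, blocks and a stealth takedown from player input or automatic reactions.
; Moves play random montages, lock movement and set attack/defense flags until finished.
; AttackZone overlaps randomly block or dodge attacking MasterCharacters, and punch or kick defending ones.
; TakedownArea enables takedowns, which line-trace a victim, snap the attacker behind it, reattach the camera boom and play paired montages before destroying the victim.
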(event `self.ReceiveActorBeginOverlap`
  (params (OtherActor :type "Actor Object Reference"))
  ;[1 1 1] Interact with overlapped Actor
  (bind _asunarmed_combat_master (cast `/Game/MyContent/Blueprints/Characters/UnarmedCombatMaster` OtherActor))
  (if (`/Game/MyContent/Blueprints/Characters/MasterCharacter.IsAttacking?` _asunarmed_combat_master)
    (`GameplayStatics.PlaySoundAtLocation` "/Game/MyContent/Audio/GroanImpact_Cue.GroanImpact_Cue" (`self.K2_GetActorLocation`) (struct) 1.0 1.0 0.0 null null null)))

(event `self.ReceiveBeginPlay`
  ;[1 1 1] BeginPlay
  (`parent.ReceiveBeginPlay`))

(event `PunchEvent`
  (bind _charactermovement (`self.CharacterMovement`))
  ;[1 1 1] Punch
  (if (`NavMovementComponent.IsFalling` (`self.CharacterMovement`)) :!label _label
    _
    (elif (not (`self.isPunching?`))
      (set `self.IsAttacking?` true)
      (set `self.isPunching?` true)
      (`CharacterMovementComponent.DisableMovement` _charactermovement)
      (bind _returnvalue (`self.PlayAnimMontage` (`|GetArrayItem` (`self.PunchAnimMontage`) (`KismetMathLibrary.RandomIntegerInRange` 0 4))))
      (`KismetSystemLibrary.Delay` _returnvalue)
      (`CharacterMovementComponent.SetMovementMode` _charactermovement "MOVE_Walking" 0)
      (set `self.isPunching?` false)
      (set `self.IsAttacking?` false))))

(event `InputAction|Punch`
  (params (Key :type "Key Structure"))
  ;[1 1 1] Punch
  (:`Pressed`
    (goto _label)))

(event `KickEvent`
  (bind _charactermovement (`self.CharacterMovement`))
  ;[1 1 1] Kick
  (if (`NavMovementComponent.IsFalling` (`self.CharacterMovement`)) :!label _label_2
    _
    (elif (not (`self.isKicking?`))
      (set `self.IsAttacking?` true)
      (set `self.isKicking?` true)
      (`CharacterMovementComponent.DisableMovement` _charactermovement)
      (bind _returnvalue (`self.PlayAnimMontage` (`|GetArrayItem` (`self.KickAnimMontage`) (`KismetMathLibrary.RandomIntegerInRange` 0 (`KismetArrayLibrary.Array_Length` (`self.KickAnimMontage`))))))
      (`KismetSystemLibrary.Delay` _returnvalue)
      (`CharacterMovementComponent.SetMovementMode` _charactermovement "MOVE_Walking" 0)
      (set `self.isKicking?` false)
      (set `self.IsAttacking?` false))))

(event `InputAction|Kick`
  (params (Key :type "Key Structure"))
  ;[1 1 1] Kick
  (:`Pressed`
    (goto _label_2)))

(event `DodgeEvent`
  (bind _charactermovement (`self.CharacterMovement`))
  ;[1 1 1] Evading
  (if (`NavMovementComponent.IsFalling` (`self.CharacterMovement`)) :!label _label_3
    _
    (elif (not (`self.IsEvading?`))
      (set `self.IsEvading?` true)
      (set `self.IsDefending?` true)
      (`CharacterMovementComponent.DisableMovement` _charactermovement)
      (bind _returnvalue (`self.PlayAnimMontage` (`|GetArrayItem` (`self.DodgeAnimMontage`) (`KismetMathLibrary.RandomIntegerInRange` 0 4))))
      (`KismetSystemLibrary.Delay` _returnvalue)
      (`CharacterMovementComponent.SetMovementMode` _charactermovement "MOVE_Walking" 0)
      (set `self.IsEvading?` false)
      (set `self.IsDefending?` false))))

(event `Dodge`
  ;[1 1 1] Evading
  (goto _label_3))

(event `BlockEvent`
  (bind _charactermovement (`self.CharacterMovement`))
  ;[1 1 1] Block
  (if (`NavMovementComponent.IsFalling` (`self.CharacterMovement`)) :!label _label_4
    _
    (elif (not (`self.IsBlocking?`))
      (set `self.IsBlocking?` false)
      (set `self.IsDefending?` true)
      (`CharacterMovementComponent.DisableMovement` _charactermovement)
      (bind _returnvalue (`self.PlayAnimMontage` (`|GetArrayItem` (`self.BlockAnimMontage`) (`KismetMathLibrary.RandomIntegerInRange` 0 4))))
      (`KismetSystemLibrary.Delay` _returnvalue)
      (`CharacterMovementComponent.SetMovementMode` _charactermovement "MOVE_Walking" 0)
      (set `self.IsBlocking?` false)
      (set `self.IsDefending?` false))))

(event `Block`
  ;[1 1 1] Block
  (goto _label_4))

(event `self.TakedownArea.OnComponentBeginOverlap`
  (params (OverlappedComponent :type "PrimitiveComponent Object Reference") (OtherActor :type "Actor Object Reference") (OtherComp :type "PrimitiveComponent Object Reference") (OtherBodyIndex :type Integer) (bFromSweep :type Boolean) (SweepResult :type "HitResult Structure (by ref)"))
  ;[1 1 1] Target character for Takedown within proximity
  (bind _asunarmed_combat_master (cast `/Game/MyContent/Blueprints/Characters/UnarmedCombatMaster` OtherActor))
  (set `/Game/MyContent/Blueprints/Characters/UnarmedCombatMaster.CanTakeDown?` true _asunarmed_combat_master))

(event `TakedownSequence`
  ;[1 1 1] Takedown Sequence
  (`CharacterMovementComponent.DisableMovement` (`self.CharacterMovement`))
  (`self.SetActorEnableCollision` false)
  (`self.PlayAnimMontage` "/Game/MyContent/Animations/Takedown/AssassinationEnemy_Montage.AssassinationEnemy_Montage")
  (`KismetSystemLibrary.Delay` 10.0)
  (`self.K2_DestroyActor`))

(event `self.TakedownArea.OnComponentEndOverlap`
  (params (OverlappedComponent :type "PrimitiveComponent Object Reference") (OtherActor :type "Actor Object Reference") (OtherComp :type "PrimitiveComponent Object Reference") (OtherBodyIndex :type Integer))
  ;[1 1 1] Target character for Takedown within proximity
  (bind _asunarmed_combat_master (cast `/Game/MyContent/Blueprints/Characters/UnarmedCombatMaster` OtherActor))
  (set `/Game/MyContent/Blueprints/Characters/UnarmedCombatMaster.CanTakeDown?` false _asunarmed_combat_master))

(event `InputAction|Takedown`
  (params (Key :type "Key Structure"))
  (bind _returnvalue (`self.K2_GetActorLocation`))
  (bind _takedowntarget (`self.TakedownTarget`))
  (bind (_returnvalue_location _returnvalue_rotation) (`KismetMathLibrary.BreakTransform` (`self.GetTransform` _takedowntarget)))
  ;[1 1 1] Perform takedown
  (:`Pressed`
    (if (`self.CanTakeDown?`)
      (bind (_outhit _returnvalue_2) (`KismetSystemLibrary.LineTraceSingle` _returnvalue (+ _returnvalue (* (`self.GetActorForwardVector`) 250.0)) "TraceTypeQuery1"))
      (if _returnvalue_2
        (bind _asunarmed_combat_master (cast `/Game/MyContent/Blueprints/Characters/UnarmedCombatMaster` (`.HitActor` (`GameplayStatics.BreakHitResult` _outhit))))
        (set `self.TakedownTarget` _asunarmed_combat_master)
        (`SceneComponent.K2_AttachToComponent` (`self.CameraBoom`) (`self.Mesh`) "spine_02" "SnapToTarget" "SnapToTarget" "SnapToTarget" true)
        (`CharacterMovementComponent.DisableMovement` (`self.CharacterMovement`))
        (set `self.CanTakeDown?` false)
        (`self.K2_SetActorTransform` (`KismetMathLibrary.MakeTransform` (+ _returnvalue_location (* (`self.GetActorForwardVector` _takedowntarget) -175.0)) _returnvalue_rotation))
        (bind _returnvalue_3 (`self.PlayAnimMontage` "/Game/MyContent/Animations/Takedown/AssassinationAttacker_Montage.AssassinationAttacker_Montage"))
        (`self.TakedownSequence` (`self.TakedownTarget`))
        (`KismetSystemLibrary.Delay` (+ _returnvalue_3 0.025))
        (`self.K2_SetActorLocation` (+ (`self.K2_GetActorLocation`) (* (`self.GetActorForwardVector`) 175.0)))
        (`CharacterMovementComponent.SetMovementMode` (`self.CharacterMovement`) "MOVE_Walking" 0)
        (`SceneComponent.K2_AttachToComponent` (`self.CameraBoom`) (`self.CapsuleComponent`) "None" "KeepRelative" "KeepRelative" "KeepRelative" true)))))

(event `self.AttackZone.OnComponentBeginOverlap`
  (params (OverlappedComponent :type "PrimitiveComponent Object Reference") (OtherActor :type "Actor Object Reference") (OtherComp :type "PrimitiveComponent Object Reference") (OtherBodyIndex :type Integer) (bFromSweep :type Boolean) (SweepResult :type "HitResult Structure (by ref)"))
  ;[1 1 1] Check Character not already attacking or defending
  (if (not (or (`self.IsAttacking?`) (`self.IsDefending?`)))
    (bind _asmaster_character (cast `/Game/MyContent/Blueprints/Characters/MasterCharacter` OtherActor))
    (`|ExecutionSequence`
      (:`then_0`
        ;[1 1 1] Opponent is attacking, Block or Dodge
        (if (`/Game/MyContent/Blueprints/Characters/MasterCharacter.IsAttacking?` _asmaster_character)
          (switch `int` (`KismetMathLibrary.RandomIntegerInRange` 0 1)
            (:`0`
              (`self.Block`))
            (:`1`
              (`self.Dodge`)))))
      (:`then_1`
        ;[1 1 1] Opponent is Defending, Punch or Kick
        (if (`/Game/MyContent/Blueprints/Characters/MasterCharacter.IsDefending?` _asmaster_character)
          (switch `int` (`KismetMathLibrary.RandomIntegerInRange` 0 1)
            (:`0`
              (`self.PunchEvent`))
            (:`1`
              (`self.KickEvent`))))))))

(fn `UserConstructionScript`
  (`parent.UserConstructionScript`))