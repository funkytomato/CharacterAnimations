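; Armed character Blueprint that carries primary, secondary and sidearm guns and handles switching, shooting, aiming and reloading.
; EquipGun shows the selected child-actor gun and snaps it to the mesh's WeaponSocket.
; EquippedGun is set only from the primary gun at construction, so shooting and reloading always target it regardless of selection.
; Aim input drives animation Blueprint flags; Threatened sets a danger flag, and SpawnProjectile spawns projectiles at the socket.
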(event `self.ReceiveBeginPlay`
  ;[1 1 1] BeginPlay - Equip Weapon and get animation reference
  (`parent.ReceiveBeginPlay`)
  (`self.SelectPrimaryWeapon`)
  (bind _asmaster_character_anim_bp (cast `/Game/MyContent/Blueprints/Characters/MasterCharacter_AnimBP` (`SkeletalMeshComponent.GetAnimInstance` (`self.Mesh`))))
  (set `self.AnimInstanceRef` _asmaster_character_anim_bp))

(event `SelectPrimaryWeapon`
  ;[1 1 1] Weapon Selection
  (set `self.CurrentlyEquipped` 0 :!label _label)
  (`self.EquipGun`))

(event `InputAction|Reload`
  (params (Key :type "Key Structure"))
  ;[1 1 1] Reload Weapon
  (:`Pressed`
    (bind _asgun_master_bp (cast `/Game/MyContent/Guns/GunMaster_BP` (`ChildActorComponent.ChildActor` (`self.PrimaryGun`))))
    (`/Game/MyContent/Guns/GunMaster_BP.Reload` _asgun_master_bp)))

(event `InputAction|PrimaryWeapon`
  (params (Key :type "Key Structure"))
  ;[1 1 1] Weapon Selection
  (:`Pressed`
    (goto _label)))

(event `InputAction|SecondaryWeapon`
  (params (Key :type "Key Structure"))
  ;[1 1 1] Weapon Selection
  (:`Pressed`
    (set `self.CurrentlyEquipped` 1)
    (`self.EquipGun`)))

(event `InputAction|SideArm`
  (params (Key :type "Key Structure"))
  ;[1 1 1] Weapon Selection
  (:`Pressed`
    (set `self.CurrentlyEquipped` 2)
    (`self.EquipGun`)))

(event `StartShooting`
  ;[1 1 1] Shooting Sequence
  (set `self.IsShooting` true :!label _label_2)
  (`/Game/MyContent/Guns/GunMaster_BP.StartShooting` (`self.EquippedGun`))
  (`|PlayMontage` (`self.Mesh`)
    (:`then`
      (`KismetSystemLibrary.PrintString` "Shooting"))))

(event `InputAction|Shoot`
  (params (Key :type "Key Structure"))
  ;[1 1 1] Shooting Sequence
  (:`Pressed`
    (goto _label_2))
  (:`Released`
    (set `self.IsShooting` false :!label _label_3)
    (`/Game/MyContent/Guns/GunMaster_BP.StopShooting` (`self.EquippedGun`))))

(event `StopShooting`
  ;[1 1 1] Shooting Sequence
  (goto _label_3))

(event `InputAction|Aim`
  (params (Key :type "Key Structure"))
  (bind _returnvalue (`SkeletalMeshComponent.GetAnimInstance` (`self.Mesh`)))
  ;[1 1 1] Aim
  (:`Pressed`
    (set `self.IsAiming?` true)
    (bind _asarmed_combat_character_anim_bp (cast `/Game/MyContent/Blueprints/Characters/ArmedCombatCharacter_AnimBP` _returnvalue))
    (set `/Game/MyContent/Blueprints/Characters/ArmedCombatCharacter_AnimBP.IsAiming` true _asarmed_combat_character_anim_bp)
    (set `/Game/MyContent/Blueprints/Characters/MasterCharacter_AnimBP.IsADS?` true _asarmed_combat_character_anim_bp))
  (:`Released`
    (set `self.IsAiming?` false)
    (bind _asarmed_combat_character_anim_bp_2 (cast `/Game/MyContent/Blueprints/Characters/ArmedCombatCharacter_AnimBP` _returnvalue))
    (set `/Game/MyContent/Blueprints/Characters/ArmedCombatCharacter_AnimBP.IsAiming` false _asarmed_combat_character_anim_bp_2)
    (set `/Game/MyContent/Blueprints/Characters/MasterCharacter_AnimBP.IsADS?` false _asarmed_combat_character_anim_bp_2)))

(event `Threatened`
  ;[1 1 1] Threatened
  (set `self.IsInDanger?` true)
  (`KismetSystemLibrary.PrintString` "Threatened!!!"))

(fn `EquipGun`
  (bind _array (`|MakeArray` (`self.PrimaryGun`) (`self.SecondaryGun`) (`self.SideArmGun`)))
  (bind _output (`|GetArrayItem` _array (`self.CurrentlyEquipped`)))
  (for _array_element _array
    (`SceneComponent.SetVisibility` _array_element false false))
  (`SceneComponent.SetVisibility` _output true false)
  (`SceneComponent.K2_AttachToComponent` _output (`self.Mesh`) "WeaponSocket" "SnapToTarget" "SnapToTarget" "SnapToTarget" true))

(fn `SpawnProjectile`
  (returns (Success :type Boolean))
  (bind _returnvalue (`|SpawnActorFromClass` "/Game/FirstPersonBP/Blueprints/FirstPersonProjectile.FirstPersonProjectile_C" (`SceneComponent.GetSocketTransform` (`self.Mesh`) "WeaponSocket" "RTS_World") "AlwaysSpawn" "OverrideRootScale" self null))
  (return (`KismetSystemLibrary.IsValid` _returnvalue)))

(fn `UserConstructionScript`
  (`parent.UserConstructionScript`)
  (bind _asgun_master_bp (cast `/Game/MyContent/Guns/GunMaster_BP` (`ChildActorComponent.ChildActor` (`self.PrimaryGun`))))
  (set `self.EquippedGun` _asgun_master_bp)
  (`SceneComponent.K2_AttachToComponent` (`self.PrimaryGun`) (`self.Mesh`) "WeaponSocket" "SnapToTarget" "SnapToTarget" "SnapToTarget" true))